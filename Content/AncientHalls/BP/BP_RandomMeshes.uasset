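; Construction-script Blueprint that lays out a grid of randomly chosen static meshes, active only when the Horizonalvertical flag is set.
; Rows, Columns and two spacing values position each cell, with shared location offset, yaw offset and scale applied.
; Each cell gets its own StaticMeshComponent rather than an instance, with a mesh drawn from MeshesUsed by unseeded random, so reconstruction reshuffles them.
; The event graph is empty.
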(event `self.ReceiveBeginPlay`)

(fn `UserConstructionScript`
  (bind _meshes_used (`self.Meshes used`))
  (if (`self.Horizonal/vertical`)
    ;[1 1 1] Setting number of instances
    (for _index (range (* (`self.rows`) (`self.Columns`)))
      ;[1 1 1] Adding mesh instances
      (bind _returnvalue (`AddComponent|NODE_AddStaticMeshComponent-0` :`RelativeTransform` (`KismetMathLibrary.MakeTransform` (+ (`self.Location offset`) (.location (`KismetMathLibrary.Conv_VectorToTransform` (`KismetMathLibrary.MakeVector` (`KismetMathLibrary.Conv_IntToDouble` (* (/ _index (`self.Columns`)) (`self.Meshes distance Columns`))) (`KismetMathLibrary.Conv_IntToDouble` (* (mod _index (`self.Columns`)) (`self.Meshes distance Rows`))))))) (`KismetMathLibrary.MakeRotator` (.roll (.rotation (`KismetMathLibrary.Conv_VectorToTransform` (`KismetMathLibrary.MakeVector` (`KismetMathLibrary.Conv_IntToDouble` (* (/ _index (`self.Columns`)) (`self.Meshes distance Columns`))) (`KismetMathLibrary.Conv_IntToDouble` (* (mod _index (`self.Columns`)) (`self.Meshes distance Rows`))))))) (.pitch (.rotation (`KismetMathLibrary.Conv_VectorToTransform` (`KismetMathLibrary.MakeVector` (`KismetMathLibrary.Conv_IntToDouble` (* (/ _index (`self.Columns`)) (`self.Meshes distance Columns`))) (`KismetMathLibrary.Conv_IntToDouble` (* (mod _index (`self.Columns`)) (`self.Meshes distance Rows`))))))) (+ (.yaw (.rotation (`KismetMathLibrary.Conv_VectorToTransform` (`KismetMathLibrary.MakeVector` (`KismetMathLibrary.Conv_IntToDouble` (* (/ _index (`self.Columns`)) (`self.Meshes distance Columns`))) (`KismetMathLibrary.Conv_IntToDouble` (* (mod _index (`self.Columns`)) (`self.Meshes distance Rows`))))))) (`self.z rotation offset`))) (* (.scale (`KismetMathLibrary.Conv_VectorToTransform` (`KismetMathLibrary.MakeVector` (`KismetMathLibrary.Conv_IntToDouble` (* (/ _index (`self.Columns`)) (`self.Meshes distance Columns`))) (`KismetMathLibrary.Conv_IntToDouble` (* (mod _index (`self.Columns`)) (`self.Meshes distance Rows`)))))) (`self.scale`)))))
      (`StaticMeshComponent.SetStaticMesh` _returnvalue (`|GetArrayItem` _meshes_used (`KismetMathLibrary.RandomIntegerInRange` 0 (`KismetArrayLibrary.Array_LastIndex` _meshes_used)))))))