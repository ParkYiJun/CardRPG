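; BP_Floors is a level-building actor that tiles an instanced mesh in a configurable rows-by-columns grid, either horizontal (XY) or vertical (XZ).
; The construction script derives each cell from the loop index, applying spacing, offset, scale and yaw with optional unseeded randomness.
; Horizontal grids can also spawn a configurable point light per instance at a height offset, apparently for chandeliers.
; The event graph has no runtime logic.
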(event `self.ReceiveBeginPlay`)

(fn `UserConstructionScript`
  (if (`self.Horizonal/vertical`)
    ;[1 1 1] Setting number of instances
    (for _index (range (* (`self.rows`) (`self.Columns`)))
      (bind _returnvalue (+ (`self.Location offset`) (.location (`KismetMathLibrary.Conv_VectorToTransform` (`KismetMathLibrary.MakeVector` (`KismetMathLibrary.Conv_IntToDouble` (* (/ _index (`self.Columns`)) (`self.Meshes distance Columns`))) (`KismetMathLibrary.Conv_IntToDouble` (* (mod _index (`self.Columns`)) (`self.Meshes distance Rows`))))))))
      ;[1 1 1] Adding mesh instances
      (`InstancedStaticMeshComponent.AddInstance` (`self.MeshUsed`) (`KismetMathLibrary.MakeTransform` _returnvalue (`KismetMathLibrary.MakeRotator` (.roll (.rotation (`KismetMathLibrary.Conv_VectorToTransform` (`KismetMathLibrary.MakeVector` (`KismetMathLibrary.Conv_IntToDouble` (* (/ _index (`self.Columns`)) (`self.Meshes distance Columns`))) (`KismetMathLibrary.Conv_IntToDouble` (* (mod _index (`self.Columns`)) (`self.Meshes distance Rows`))))))) (.pitch (.rotation (`KismetMathLibrary.Conv_VectorToTransform` (`KismetMathLibrary.MakeVector` (`KismetMathLibrary.Conv_IntToDouble` (* (/ _index (`self.Columns`)) (`self.Meshes distance Columns`))) (`KismetMathLibrary.Conv_IntToDouble` (* (mod _index (`self.Columns`)) (`self.Meshes distance Rows`))))))) (+ (.yaw (.rotation (`KismetMathLibrary.Conv_VectorToTransform` (`KismetMathLibrary.MakeVector` (`KismetMathLibrary.Conv_IntToDouble` (* (/ _index (`self.Columns`)) (`self.Meshes distance Columns`))) (`KismetMathLibrary.Conv_IntToDouble` (* (mod _index (`self.Columns`)) (`self.Meshes distance Rows`))))))) (+ (`self.z rotation offset`) (* (`KismetMathLibrary.RandomFloatInRange` -359.0 359.0) (`self.Z Rotation Randomness`))))) (* (.scale (`KismetMathLibrary.Conv_VectorToTransform` (`KismetMathLibrary.MakeVector` (`KismetMathLibrary.Conv_IntToDouble` (* (/ _index (`self.Columns`)) (`self.Meshes distance Columns`))) (`KismetMathLibrary.Conv_IntToDouble` (* (mod _index (`self.Columns`)) (`self.Meshes distance Rows`)))))) (`self.scale`))))
      (if (`self.Add Point Light (chandelier)`)
        (bind _returnvalue_2 (`AddComponent|NODE_AddPointLightComponent-0` :`RelativeTransform` (`KismetMathLibrary.MakeTransform` (+ _returnvalue (`KismetMathLibrary.MakeVector` 0.0 0.0 (`self.Light height offset`))))))
        (`LightComponentBase.SetCastShadows` _returnvalue_2 (`self.Light casts shadows`))
        (`LightComponent.SetIntensity` _returnvalue_2 (`self.Light intensity`))
        (`PointLightComponent.SetAttenuationRadius` _returnvalue_2 (`self.Light Radius`))))
    (else
      (for _index_2 (range (* (`self.rows`) (`self.Columns`)))
        (`InstancedStaticMeshComponent.AddInstance` (`self.MeshUsed`) (`KismetMathLibrary.MakeTransform` (+ (`self.Location offset`) (.location (`KismetMathLibrary.Conv_VectorToTransform` (`KismetMathLibrary.MakeVector` (`KismetMathLibrary.Conv_IntToDouble` (* (/ _index_2 (`self.Columns`)) (`self.Meshes distance Columns`))) 0.0 (`KismetMathLibrary.Conv_IntToDouble` (* (mod _index_2 (`self.Columns`)) (`self.Meshes distance Rows`))))))) (`KismetMathLibrary.MakeRotator` (.roll (.rotation (`KismetMathLibrary.Conv_VectorToTransform` (`KismetMathLibrary.MakeVector` (`KismetMathLibrary.Conv_IntToDouble` (* (/ _index_2 (`self.Columns`)) (`self.Meshes distance Columns`))) 0.0 (`KismetMathLibrary.Conv_IntToDouble` (* (mod _index_2 (`self.Columns`)) (`self.Meshes distance Rows`))))))) (.pitch (.rotation (`KismetMathLibrary.Conv_VectorToTransform` (`KismetMathLibrary.MakeVector` (`KismetMathLibrary.Conv_IntToDouble` (* (/ _index_2 (`self.Columns`)) (`self.Meshes distance Columns`))) 0.0 (`KismetMathLibrary.Conv_IntToDouble` (* (mod _index_2 (`self.Columns`)) (`self.Meshes distance Rows`))))))) (+ (.yaw (.rotation (`KismetMathLibrary.Conv_VectorToTransform` (`KismetMathLibrary.MakeVector` (`KismetMathLibrary.Conv_IntToDouble` (* (/ _index_2 (`self.Columns`)) (`self.Meshes distance Columns`))) 0.0 (`KismetMathLibrary.Conv_IntToDouble` (* (mod _index_2 (`self.Columns`)) (`self.Meshes distance Rows`))))))) (+ (`self.z rotation offset`) (* (`KismetMathLibrary.RandomFloatInRange` -359.0 359.0) (`self.Z Rotation Randomness`))))) (* (.scale (`KismetMathLibrary.Conv_VectorToTransform` (`KismetMathLibrary.MakeVector` (`KismetMathLibrary.Conv_IntToDouble` (* (/ _index_2 (`self.Columns`)) (`self.Meshes distance Columns`))) 0.0 (`KismetMathLibrary.Conv_IntToDouble` (* (mod _index_2 (`self.Columns`)) (`self.Meshes distance Rows`)))))) (`self.scale`))))))))