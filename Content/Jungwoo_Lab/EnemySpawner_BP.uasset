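; Enemy spawner actor that spawns BP_Bear at random intervals once ActivateSpawner is called.
; A looping delay picks a random SpawnPoints entry, or its own transform if spawn points are disabled, and spawns slightly above it.
; Count limits spawns, with -1 looping endlessly; when exhausted, the spawner destroys itself after a short delay.
; BeginPlay iterates SpawnPoint actors but does nothing with them.
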(event `self.ReceiveBeginPlay`
  (`|ExecutionSequence`
    (:`then_0`
      (if (`self.UseSpawnPoint`)
        (bind _outactors (`GameplayStatics.GetAllActorsOfClass` "/Game/Jungwoo_Lab/SpawnPoint.SpawnPoint_C"))
        (for _ _outactors
          (if true
            _))))))

(event `StartSpawning`
  (bind (_spawnlocation_location _spawnlocation_rotation) (`KismetMathLibrary.BreakTransform` (`self.SpawnLocation`)))
  (`KismetSystemLibrary.Delay` (`KismetMathLibrary.RandomFloatInRange` (`self.SpawnDelay_Min`) (`self.SpawnDelay_Max`)) :!label _label)
  (if (`self.UseSpawnPoint`)
    (if (== (`KismetArrayLibrary.Array_Length` (`self.SpawnPoints`)) 1)
      (set `self.SpawnLocation` (`self.GetTransform` (`|GetArrayItem` (`self.SpawnPoints`))))
      (else
        (set `self.SpawnLocation` (`self.GetTransform` (`|GetArrayItem` (`self.SpawnPoints`) (`KismetMathLibrary.RandomIntegerInRange` 0 (- (`KismetArrayLibrary.Array_Length` (`self.SpawnPoints`)) 1)))))))
    (else
      (set `self.SpawnLocation` (`self.GetTransform`))))
  (`|SpawnActorFromClass` "/Game/InfinityBladeAdversaries/AI/lab/BP_Bear.BP_Bear_C" (`KismetMathLibrary.MakeTransform` (+ _spawnlocation_location (0.0 0.0 3.0)) _spawnlocation_rotation) "Undefined" "OverrideRootScale" null null)
  (if (== (`self.Count`) -1)
    (goto _label)
    (else
      (set `self.Count` (- (`self.Count`) 1))
      (if (> (`self.Count`) 0)
        (goto _label)
        (else
          (`KismetSystemLibrary.Delay` 0.5)
          (`self.K2_DestroyActor`))))))

(event `ActivateSpawner`
  (`self.StartSpawning`))

(fn `UserConstructionScript`)