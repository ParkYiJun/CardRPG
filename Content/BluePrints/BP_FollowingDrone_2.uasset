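; BP_FollowingDrone_2 is a drone that follows the main character around the level.
; On BeginPlay it casts the player character to BP_MainCharacter and stores the reference.
; A looping FollowPlayer event uses AI MoveTo toward the world location of the character's Ddrone component, re-issuing the move after a short delay to track the moving target.
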(event `self.ReceiveBeginPlay`
  (bind _asbp_main_character (cast `/Game/BluePrints/BP_MainCharacter` (`GameplayStatics.GetPlayerCharacter` 0)))
  (set `self.As BP Main Character` _asbp_main_character)
  (`self.FollowPlayer`))

(event `FollowPlayer`
  (`|AIMoveTo` self (`SceneComponent.K2_GetComponentLocation` (`/Game/BluePrints/BP_MainCharacter.Ddrone` (`self.As BP Main Character`))) null 15.0
    (:`then`
      (`KismetSystemLibrary.Delay` 0.1)
      (`self.FollowPlayer`))))

(fn `UserConstructionScript`)