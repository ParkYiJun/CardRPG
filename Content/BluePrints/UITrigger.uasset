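; UITrigger is a trigger actor that plays a media clip behind a paused game when BP_MainCharacter overlaps it.
; On overlap it links MediaSound to the media player, pauses the game, adds a widget to the viewport and opens the media source.
; When playback reaches its end, the bound End event unpauses and destroys the trigger, making it one-shot; the widget is not removed here.
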(event `self.ReceiveActorBeginOverlap`
  (params (OtherActor :type "Actor Object Reference"))
  (bind _media (`self.Media`))
  (cast `/Game/BluePrints/BP_MainCharacter` OtherActor)
  (`MediaSoundComponent.SetMediaPlayer` (`self.MediaSound`) (`self.Media`))
  (`GameplayStatics.SetGamePaused` true)
  (bind _returnvalue (`|CreateWidget` (`self.Widget`) (`GameplayStatics.GetPlayerController` 0)))
  (`UserWidget.AddToViewport` _returnvalue 0)
  (`MediaPlayer.OpenSource` _media (`self.mediaSource`))
  (add `MediaPlayer.OnEndReached` _media (delegate `End`)))

(event `End`
  (`GameplayStatics.SetGamePaused` false)
  (`self.K2_DestroyActor`))

(fn `UserConstructionScript`)